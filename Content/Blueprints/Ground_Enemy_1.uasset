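; Ground_Enemy_1 is a Paper2D ground enemy that can be grappled and shows a stunned flipbook while held.
; It takes damage from a Drill_Enemy's drill hitbox and damages other PaperEnemy actors it hits while falling.
; Tick handles death by disabling collision, playing explosion sound and animation, then destroying the actor.
; A timeline patrol between two points is set up on BeginPlay but never runs.
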(event OnComponentHit(CapsuleComponent)
  (params (OtherActor :type Actor%20Object%20Reference) (OtherComp :type Primitive%20Component%20Object%20Reference) (NormalImpulse :type Vector :default "0, 0, 0") (Hit :type Hit%20Result%20Structure%20%28by%20ref%29))
  (if (and (Utilities|ClassIsChildOf (Utilities|GetClass OtherActor) "/Script/EggletonProject.PaperEnemy") (AI|Components|NavMovement|IsFalling (Variables|Character|GetCharacterMovement)))
    (Game|Damage|ApplyDamage OtherActor 1.0 0 0)))

(event EventHit
  (params (MyComp :type Primitive%20Component%20Object%20Reference) (Other :type Actor%20Object%20Reference) (OtherComp :type Primitive%20Component%20Object%20Reference) (bSelfMoved :type Boolean) (HitLocation :type Vector :default "0, 0, 0") (HitNormal :type Vector :default "0, 0, 0") (NormalImpulse :type Vector :default "0, 0, 0") (Hit :type Hit%20Result%20Structure%20%28by%20ref%29))
  (bind _asdrill_enemy_c (Utilities|Casting|CastToDrill_Enemy Other))
  (if (== (Variables|/Game/Blueprints/Drill_Enemy.Drill_Enemy_C|GetDrillHitBox _asdrill_enemy_c) OtherComp)
    (Game|Damage|ApplyDamage 0 3.0 0 0)))

(event EventAnyDamage
  (params (Damage :type Float%20%28single-precision%29) (DamageType :type Damage%20Type%20Object%20Reference) (InstigatedBy :type Controller%20Object%20Reference) (DamageCauser :type Actor%20Object%20Reference))
  (Variables|Default|SetCurrentHealth (- (Variables|Default|GetCurrentHealth) (Math|Float|Floor Damage))))

(event EventTick
  (params (DeltaSeconds :type Float%20%28single-precision%29))
  (bind _capsulecomponent (Variables|Default|GetCapsuleComponent))
  (if (<= (Variables|Default|GetCurrentHealth) 0)
    (if (Variables|Default|GetIsDead)
      (if (>= (Components|Timeline|GetPlaybackPosition (Variables|Default|GetSprite)) 0.45)
        (Actor|DestroyActor))
      (else
        (Variables|Default|SetIsDead true)
        (Collision|SetCollisionEnabled _capsulecomponent "NoCollision")
        (Sprite|SetFlipbook (Variables|Default|GetSprite) (Variables|Default|GetDeath_Anim))
        (Class|GameplayStatics|PlaySoundAttached "/Game/Audio/Sound_Effects/Explosion.Explosion" _capsulecomponent)))
    (elif (Variables|Default|GetIsGrappled)
      (Sprite|SetFlipbook (Variables|Default|GetSprite) (Variables|Default|GetStunned_Anim))
      (Pawn|Components|CharacterMovement|SetMovementMode (Variables|Character|GetCharacterMovement) "MOVE_Walking" 0))))

(event EventBeginPlay
  ;[1 1 1] Unused Patrol routes
  (Variables|Default|SetHasPatrolPoints (and (Utilities|IsValid (Variables|Default|GetStartPoint)) (Utilities|IsValid (Variables|Default|GetEndPoint))))
  (if (Variables|Default|GetHasPatrolPoints)
    (Variables|Default|SetPatrolDist (CallFunction|DistBetweenPatrolPoints (Variables|Default|GetStartPoint) (Variables|Default|GetEndPoint)))
    (if (<= (/ (Variables|Default|GetPatrolDist) 1e+03) 1.0)
      (Variables|Default|SetPatrolRate (/ (Variables|Default|GetPatrolDist) 1e+03))
      (Components|Timeline|SetPlayRate (Variables|Default|GetPatrolRoute) 0.5)
      (else
        (Components|Timeline|SetPlayRate (Variables|Default|GetPatrolRoute) 1.0)))))

(fn ConstructionScript
  (Variables|Default|SetVerticalLerpOffset 31.0))

(fn DistBetweenPatrolPoints
  (params (Point1 :type Actor%20Object%20Reference) (Point2 :type Actor%20Object%20Reference))
  (LocalVariables|SetPoint1_L Point1)
  (LocalVariables|SetPoint2_L Point2)
  (return (Math|Float|Sqrt (+ (Math|Float|Square (- (.X (Math|Vector|BreakVector (Transformation|GetActorLocation (LocalVariables|GetPoint1_L)))) (.X (Math|Vector|BreakVector (Transformation|GetActorLocation (LocalVariables|GetPoint2_L)))))) (Math|Float|Square (- (.Z (Math|Vector|BreakVector (Transformation|GetActorLocation (LocalVariables|GetPoint1_L)))) (.Z (Math|Vector|BreakVector (Transformation|GetActorLocation (LocalVariables|GetPoint2_L))))))))))