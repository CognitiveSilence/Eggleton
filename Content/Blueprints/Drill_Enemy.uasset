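; Drill enemy for a 2D Paper sprite game that drops 300 units when an EggPlayer or PaperEnemy enters its trigger.
; A timeline lerps the drop, then starts a timeline patrol between two placed points, flipping the sprite at the ends.
; BeginPlay sets patrol speed from point distance in the XZ plane.
; Damage reduces health, and Tick handles death animation, sound and destruction; grapple-stun logic is left disconnected.
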(event OnComponentBeginOverlap(DropTrigger)
  (params (OtherActor :type Actor%20Object%20Reference) (OtherComp :type Primitive%20Component%20Object%20Reference) (OtherBodyIndex :type Integer) (bFromSweep :type Boolean) (SweepResult :type Hit%20Result%20Structure%20%28by%20ref%29))
  (bind _returnvalue (Utilities|GetClass OtherActor))
  (if (and (not (Variables|DrillDrop|GetIsDropping)) (or (Utilities|ClassIsChildOf _returnvalue "/Game/Blueprints/EggPlayer.EggPlayer_C") (Utilities|ClassIsChildOf _returnvalue "/Script/EggletonProject.PaperEnemy")))
    (Variables|DrillDrop|SetIsDropping true)
    (Variables|DrillDrop|SetvDropTargetLocation (- (Transformation|GetActorLocation) (Math|Vector|MakeVector 0.0 0.0 3e+02)))
    (Variables|DrillDrop|SetvLocationBeforeDrop (Transformation|GetActorLocation))
    (CallFunction|BeginDrop)))

(event Custom|Patrol
  (bind _sprite (Variables|Default|GetSprite))
  ;[1 1 1] Patrol Routes
  (bind _patrolval (Timeline|PatrolRoute Play)
    (:Update
      (if (Math|Boolean|ORBoolean (not (Variables|Default|GetHasPatrolPoints)) (Variables|Default|GetIsGrappled) (Variables|Default|GetIsDead) (Variables|DrillDrop|GetIsDropping))
        (Timeline|PatrolRoute Stop)
        (else
          (Transformation|SetActorLocation self (Math|Vector|Lerp(Vector) (Transformation|GetActorLocation (Variables|Default|GetStartPoint)) (Transformation|GetActorLocation (Variables|Default|GetEndPoint)) _patrolval) false)
          (if (>= _patrolval 0.9)
            (Transformation|SetWorldScale3D _sprite "-1.000000,1.000000,1.000000")
            (elif (<= _patrolval 0.0)
              (Transformation|SetWorldScale3D _sprite "1.000000,1.000000,1.000000"))))))))

(event Custom|BeginDrop
  (bind _dropval (Timeline|Drop PlayFromStart)
    (:Update
      (Transformation|SetActorLocation (Math|Vector|Lerp(Vector) (Variables|DrillDrop|GetvLocationBeforeDrop) (Variables|DrillDrop|GetvDropTargetLocation) _dropval) false))
    (:Finished
      (Development|PrintString "Hello")
      (Variables|DrillDrop|SetIsDropping false)
      (CallFunction|Patrol))))

(event EventAnyDamage
  (params (Damage :type Float%20%28single-precision%29) (DamageType :type Damage%20Type%20Object%20Reference) (InstigatedBy :type Controller%20Object%20Reference) (DamageCauser :type Actor%20Object%20Reference))
  ;[1 1 1] Receive Damage
  (Variables|Default|SetCurrentHealth (- (Variables|Default|GetCurrentHealth) (Math|Float|Floor Damage))))

(event EventTick
  (params (DeltaSeconds :type Float%20%28single-precision%29))
  ;[1 1 1] Check if Alive
  (if (<= (Variables|Default|GetCurrentHealth) 0)
    (if (Variables|Default|GetIsDead)
      ;[1 1 1] Wait until Death Anim finishes before destroying self
      (if (>= (Components|Timeline|GetPlaybackPosition (Variables|Default|GetSprite)) 0.45)
        (Actor|DestroyActor))
      (else
        ;[1 1 1] Start death animation and sound
        (Variables|Default|SetIsDead true)
        (Collision|SetCollisionEnabled (Variables|Default|GetCapsuleComponent) "NoCollision")
        (Sprite|SetFlipbook (Variables|Default|GetSprite) (Variables|Default|GetDeath_Anim))
        (Class|GameplayStatics|PlaySoundAttached "/Game/Audio/Sound_Effects/Explosion.Explosion" (Variables|Default|GetCapsuleComponent))))))

(event EventBeginPlay
  ;[1 1 1] Patrol Routes
  (Variables|Default|SetHasPatrolPoints (and (Utilities|IsValid (Variables|Default|GetStartPoint)) (Utilities|IsValid (Variables|Default|GetEndPoint))))
  (if (Variables|Default|GetHasPatrolPoints)
    (Variables|Default|SetPatrolDist (CallFunction|DistBetweenPatrolPoints (Variables|Default|GetStartPoint) (Variables|Default|GetEndPoint)))
    (if (<= (/ (Variables|Default|GetPatrolDist) 1e+03) 1.0)
      (Variables|Default|SetPatrolRate (/ (Variables|Default|GetPatrolDist) 1e+03))
      (Components|Timeline|SetPlayRate (Variables|Default|GetPatrolRoute) 1.0)
      (else
        (Components|Timeline|SetPlayRate (Variables|Default|GetPatrolRoute) 0.5)))))

(fn ConstructionScript
  (Variables|Default|SetVerticalLerpOffset 31.0))

(fn DistBetweenPatrolPoints
  (params (Point1 :type Actor%20Object%20Reference) (Point2 :type Actor%20Object%20Reference))
  (LocalVariables|SetPoint1_L Point1)
  (LocalVariables|SetPoint2_L Point2)
  (return (Math|Float|Sqrt (+ (Math|Float|Square (- (.X (Math|Vector|BreakVector (Transformation|GetActorLocation (LocalVariables|GetPoint1_L)))) (.X (Math|Vector|BreakVector (Transformation|GetActorLocation (LocalVariables|GetPoint2_L)))))) (Math|Float|Square (- (.Z (Math|Vector|BreakVector (Transformation|GetActorLocation (LocalVariables|GetPoint1_L)))) (.Z (Math|Vector|BreakVector (Transformation|GetActorLocation (LocalVariables|GetPoint2_L))))))))))