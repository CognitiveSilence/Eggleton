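; Paper2D side-scrolling player character that runs, jumps and toggles a heavy egg state, with a HUD widget showing health.
; Egg state blocks movement and jumping, turns airborne velocity into a downward slam and damages overlapped actors; otherwise overlaps hurt the player unless grappling.
; Movement input updates animation: a state function picks the flipbook from motion, facing and egg flags, and the egg animation freezes on a held frame.
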(event Custom|UpdateAnim
  ;[1 1 1] Animations
  (Variables|Default|SetIsMoving (> (Math|Vector|VectorLength (Transformation|GetVelocity)) 0.0))
  (Variables|Default|SetIsFalling (AI|Components|NavMovement|IsFalling (Variables|Character|GetCharacterMovement)))
  (bind _outflip (CallFunction|AnimationStateMachine (Variables|Default|GetIsFalling) (Variables|Default|GetIsMoving) (Variables|Default|GetEggState) (Variables|Default|GetFacingRight)))
  (Sprite|SetFlipbook (Variables|Default|GetSprite) _outflip)
  (CallFunction|PauseAnimonEggState))

(event EventActorBeginOverlap
  (params (OtherActor :type Actor%20Object%20Reference))
  ;[1 1 1] Damage (needs rework)
  (if (Variables|Default|GetEggState)
    (Game|Damage|ApplyDamage OtherActor 1.0 0 0)
    (elif (not (Variables|Default|GetIsGrappling))
      (Game|Damage|ApplyDamage self 2e+01 0 0))))

(event EventAnyDamage
  (params (Damage :type Float%20%28single-precision%29) (DamageType :type Damage%20Type%20Object%20Reference) (InstigatedBy :type Controller%20Object%20Reference) (DamageCauser :type Actor%20Object%20Reference))
  (bind _returnvalue (Math|Float|Floor Damage))
  ;[1 1 1] Damage (needs rework)
  (Variables|Default|SetCurrentHealth (- (Variables|Default|GetCurrentHealth) _returnvalue))
  (Default|SetPlayerHealth (Variables|Default|GetGameGUI) _returnvalue 100))

(event EventBeginPlay
  ;[1 1 1] Replication - MP
  (Class|ActorComponent|SetIsReplicated (Variables|Default|GetSprite) true)
  ;[1 1 1] Create UI
  (bind _returnvalue (UserInterface|CreateWidget "/Game/GUI/GameUI.GameUI_C"))
  (Variables|Default|SetGameGUI _returnvalue)
  (UserInterface|Viewport|AddtoViewport _returnvalue))

(event Input|ActionEvents|InputActionJump
  ;[1 1 1] Jumping
  (:Pressed
    (if (not (Variables|Default|GetEggState))
      (Character|Jump)
      (Class|GameplayStatics|PlaySoundAttached "/Game/Audio/Jump.Jump"))))

(event Input|ActionEvents|InputActionHeavyMode
  ;[1 1 1] Egg State
  (:Pressed
    (Utilities|FlowControl|FlipFlop
      (:A
        (Variables|Default|SetEggState true)
        (if (Variables|Default|GetIsFalling)
          (Variables|/Script/Engine.MovementComponent|SetVelocity (Variables|Character|GetCharacterMovement) (stale _returnvalue))))
      (:B
        (Variables|Default|SetEggState false)))))

(event Input|ActionEvents|InputActionLookLeft
  ;[1 1 1] Animations
  (:Pressed
    (Variables|Default|SetFacingRight false)))

(event Input|ActionEvents|InputActionLookRight
  ;[1 1 1] Animations
  (:Pressed
    (Variables|Default|SetFacingRight true)))

(event Input|AxisEvents|InputAxisMoveRight
  (params (AxisValue :type Float%20%28single-precision%29))
  ;[1 1 1] Movement
  (if (Variables|Default|GetEggState)
    (CallFunction|UpdateAnim)
    (else
      (Pawn|Input|AddMovementInput "1.000000, 0, 0" AxisValue false)
      (CallFunction|UpdateAnim))))

(fn ConstructionScript
  (Variables|Default|SetFacingRight true)
  (Variables|Animations|SetPausedOnEggFrame false))

(fn AnimationStateMachine
  (params (IsFalling :type Boolean) (IsMoving :type Boolean) (IsHeavy :type Boolean) (FacingRight :type Boolean))
  (LocalVariables|SetIsJumpingL IsFalling)
  (LocalVariables|SetIsMovingL IsMoving)
  (LocalVariables|SetIsHeavyL IsHeavy)
  (LocalVariables|SetFacingRightL FacingRight)
  (if (LocalVariables|GetIsJumpingL)
    (if (LocalVariables|GetFacingRightL)
      (LocalVariables|SetAnimationStated "NewEnumerator2")
      (else
        (LocalVariables|SetAnimationStated "NewEnumerator6")))
    (elif (LocalVariables|GetIsMovingL)
      (if (LocalVariables|GetFacingRightL)
        (LocalVariables|SetAnimationStated "NewEnumerator1")
        (else
          (LocalVariables|SetAnimationStated "NewEnumerator5")))
      (elif (LocalVariables|GetFacingRightL)
        (LocalVariables|SetAnimationStated "NewEnumerator0")
        (else
          (LocalVariables|SetAnimationStated "NewEnumerator4")))))
  (if (LocalVariables|GetIsHeavyL)
    (if (LocalVariables|GetFacingRightL)
      (LocalVariables|SetAnimationStated "NewEnumerator3")
      (else
        (LocalVariables|SetAnimationStated "NewEnumerator7"))))
  (return (Utilities|Select :Index (LocalVariables|GetAnimationStated) :NewEnumerator0 (Variables|Animations|GetIdle_Right_Flipbook) :NewEnumerator1 (Variables|Animations|GetRun_Right_Flipbook) :NewEnumerator2 (Variables|Animations|GetJump_Right_Flipbook) :NewEnumerator3 (Variables|Animations|GetHeavy_Right_Flipbook) :NewEnumerator4 (Variables|Animations|GetIdle_Left_Flipbook) :NewEnumerator5 (Variables|Animations|GetRun_Left_Flipbook) :NewEnumerator6 (Variables|Animations|GetJump_Left_Flipbook) :NewEnumerator7 (Variables|Animations|GetHeavy_Left_Flipbook))))

(fn PauseAnimonEggState
  (if (Variables|Default|GetEggState)
    (if (Variables|Animations|GetPausedOnEggFrame)
      (Components|Timeline|SetPlaybackPosition (Variables|Default|GetSprite) 0.45 false)
      (elif (>= (Components|Timeline|GetPlaybackPosition (Variables|Default|GetSprite)) 0.45)
        (Audio|Components|Audio|Stop (Variables|Default|GetSprite))
        (Variables|Animations|SetPausedOnEggFrame true)))
    (else
      (Audio|Components|Audio|Play (Variables|Default|GetSprite))
      (Variables|Animations|SetPausedOnEggFrame false)))
  (return))

(fn MakeEggVectorfromCurrentVelocity
  (return (Math|Vector|MakeVector 0.0 0.0 (* (Math|Float|Absolute(Float) (.Z (Math|Vector|BreakVector (Variables|/Script/Engine.MovementComponent|GetVelocity (Variables|Character|GetCharacterMovement))))) -3.0))))