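; Paper2D cannon enemy that turns toward the player and fires a cannonball that way every second unless grappled, with no range check.
; Tick drives shooting, death and AnimStateMachine, which flips the actor and times the return to idle by flipbook playback position; FacingRight is true when the player is not to the right.
; Damage lowers health until it explodes and is destroyed; while falling, it damages PaperEnemy actors it hits.
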(event OnComponentHit(CapsuleComponent)
  (params (OtherActor :type Actor%20Object%20Reference) (OtherComp :type Primitive%20Component%20Object%20Reference) (NormalImpulse :type Vector :default "0, 0, 0") (Hit :type Hit%20Result%20Structure%20%28by%20ref%29))
  (if (and (Utilities|ClassIsChildOf (Utilities|GetClass OtherActor) "/Script/EggletonProject.PaperEnemy") (AI|Components|NavMovement|IsFalling (Variables|Character|GetCharacterMovement)))
    (Game|Damage|ApplyDamage OtherActor 1.0 0 0)))

(event EventAnyDamage
  (params (Damage :type Float%20%28single-precision%29) (DamageType :type Damage%20Type%20Object%20Reference) (InstigatedBy :type Controller%20Object%20Reference) (DamageCauser :type Actor%20Object%20Reference))
  (Variables|Default|SetCurrentHealth (- (Variables|Default|GetCurrentHealth) (Math|Float|Floor Damage))))

(event EventTick
  (params (DeltaSeconds :type Float%20%28single-precision%29))
  (bind _capsulecomponent (Variables|Default|GetCapsuleComponent))
  (Variables|Default|SetfShoot_Countdown (- (Variables|Default|GetfShoot_Countdown) DeltaSeconds))
  (Variables|Default|SetbFacingRight (not (< (.X (Math|Vector|BreakVector (Transformation|GetActorLocation))) (.X (Math|Vector|BreakVector (Transformation|GetActorLocation (Game|Player|GetPlayerPawn 0)))))))
  (if (<= (Variables|Default|GetCurrentHealth) 0)
    (if (Variables|Default|GetIsDead)
      (if (>= (Components|Timeline|GetPlaybackPosition (Variables|Default|GetSprite)) 0.45)
        (Actor|DestroyActor))
      (else
        (Variables|Default|SetIsDead true)
        (Collision|SetCollisionEnabled _capsulecomponent "NoCollision")
        (Sprite|SetFlipbook (Variables|Default|GetSprite) (Variables|Default|GetDeath_Anim))
        (Class|GameplayStatics|PlaySoundAttached "/Game/Audio/Sound_Effects/Explosion.Explosion" _capsulecomponent)))
    (else
      (CallFunction|AnimStateMachine)
      (if (not (Variables|Default|GetIsGrappled))
        (if (<= (Variables|Default|GetfShoot_Countdown) 0.0)
          (Variables|Default|SetfShoot_Countdown 1.0)
          (if (Variables|Default|GetbFacingRight)
            (bind _returnvalue (Game|SpawnActorfromClass "/Game/Blueprints/cannonball_enemy.cannonball_enemy_C" (Math|Conversions|ToTransform(Vector) (+ (Transformation|GetActorLocation) "-150.000000,0.000000,0.000000")) true 0))
            (Variables|/Game/Blueprints/cannonball_enemy.cannonball_enemy_C|SetbMovingRight _returnvalue (Variables|Default|GetbFacingRight))
            (Variables|/Script/Engine.MovementComponent|SetVelocity (Variables|/Script/Engine.Character|GetCharacterMovement _returnvalue) "-100.000000, 0, 0")
            (else
              (bind _returnvalue_2 (Game|SpawnActorfromClass "/Game/Blueprints/cannonball_enemy.cannonball_enemy_C" (Math|Conversions|ToTransform(Vector) (+ (Transformation|GetActorLocation) "150.000000, 0,0.000000")) true 0))
              (Variables|/Game/Blueprints/cannonball_enemy.cannonball_enemy_C|SetbMovingRight _returnvalue_2 (Variables|Default|GetbFacingRight))
              (Variables|/Script/Engine.MovementComponent|SetVelocity (Variables|/Script/Engine.Character|GetCharacterMovement _returnvalue_2) "100.000000, 0, 0")))
          (bind _returnvalue_3 (Sprite|SetFlipbook (Variables|Default|GetSprite) (Variables|Default|GetShooting_Anim)))
          (Variables|Default|SetbShooting _returnvalue_3)
          (Class|GameplayStatics|PlaySoundAttached "/Game/Audio/Sound_Effects/Explosion.Explosion" (Variables|Default|GetHead) "None" "0, 0, 0" "KeepRelativeOffset" false 0.5 2.0))))))

(fn ConstructionScript
  (Variables|Default|SetVerticalLerpOffset 6.0))

(fn DistBetweenPatrolPoints
  (params (Point1 :type Actor%20Object%20Reference) (Point2 :type Actor%20Object%20Reference))
  (LocalVariables|SetPoint1_L Point1)
  (LocalVariables|SetPoint2_L Point2)
  (return (Math|Float|Sqrt (+ (Math|Float|Square (- (.X (Math|Vector|BreakVector (Transformation|GetActorLocation (LocalVariables|GetPoint1_L)))) (.X (Math|Vector|BreakVector (Transformation|GetActorLocation (LocalVariables|GetPoint2_L)))))) (Math|Float|Square (- (.Z (Math|Vector|BreakVector (Transformation|GetActorLocation (LocalVariables|GetPoint1_L)))) (.Z (Math|Vector|BreakVector (Transformation|GetActorLocation (LocalVariables|GetPoint2_L))))))))))

(fn AnimStateMachine
  (if (not (Variables|Default|GetIsDead))
    (if (Variables|Default|GetbFacingRight)
      (Transformation|SetActorRotation (Class|KismetMathLibrary|MakeRot 1.8e+02 0.0 1.8e+02))
      (else
        (Transformation|SetActorRotation (Class|KismetMathLibrary|MakeRot 0.0 0.0 0.0))))
    (if (Variables|Default|GetbShooting)
      (if (>= (Components|Timeline|GetPlaybackPosition (Variables|Default|GetSprite)) 0.49)
        (Variables|Default|SetbShooting false)
        (Sprite|SetFlipbook (Variables|Default|GetSprite) (Variables|Default|GetIdle_Anim))))))