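; A 2D sprite lift that travels between its origin and EndLocation over a configurable travel time.
; A timeline lerps the sprite's position, and on finishing waits WaitTime before calling for the opposite direction.
; A Safety trigger calls Play or Reverse on the active timeline when an EggPlayer overlaps it, based on its playing state.
; The construction script applies the lift colour and can preview the end position via TestEndLocation.
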(event `self.ReceiveBeginPlay`
  (`TimelineComponent.SetPlayRate` (`self.LiftTimeline`) (/ 1.0 (`self.TravelTimeInSeconds`)))
  (set `self.TestEndLocation` true))

(event `self.safety.OnComponentBeginOverlap`
  (params (OtherActor :type "Actor Object Reference") (OtherComp :type "PrimitiveComponent Object Reference") (OtherBodyIndex :type Integer) (bFromSweep :type Boolean) (SweepResult :type "EngineTypes.HitResult Structure (by ref)"))
  (bind _lifttimeline (`self.LiftTimeline`))
  (cast `/Game/Blueprints/EggPlayer` OtherActor)
  (if (`ActorComponent.IsActive` _lifttimeline)
    (if (`TimelineComponent.IsPlaying` _lifttimeline)
      (bind (_direction _driver) (`Timeline|LiftTimeline` :!label _label)
        (:`Update`
          (`SceneComponent.SetRelativeLocation` (`self.LiftSprite`) (`KismetMathLibrary.VLerp` (0.0 0.0 0.0) (`self.EndLocation`) _driver) false))
        (:`Finished`
          (`KismetSystemLibrary.Delay` (`self.WaitTime`))
          (switch `TimelineComponent.ETimelineDirection` _direction
            (:`Forward`
              (`self.Lift_Backward`))
            (:`Backward`
              (`self.Lift_Forward`)))))
      (else
        (goto _label :!via `Reverse`)))))

(event `Lift_Forward`
  (goto _label :!via `PlayFromStart`))

(event `Lift_Backward`
  (goto _label :!via `ReverseFromEnd`))

(fn `UserConstructionScript`
  (bind _liftsprite (`self.LiftSprite`))
  (`SceneComponent.SetRelativeLocation` _liftsprite (`KismetMathLibrary.SelectVector` (`self.EndLocation`) (0.0 0.0 0.0) (`self.TestEndLocation`)) false)
  (`PaperSpriteComponent.SetSpriteColor` _liftsprite (`self.LiftColour`)))