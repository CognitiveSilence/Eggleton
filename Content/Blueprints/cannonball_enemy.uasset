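; Enemy cannonball projectile that flies forward and damages what it strikes.
; Tick forces half-scale movement input along the actor's forward vector, using character movement rather than a projectile component.
; On hit, it damages EggPlayer or PaperEnemy actors, then plays a landing sound and destroys itself whatever it struck.
; Unconnected leftover nodes hold a low-speed debug check and direction-based velocity logic.
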(event `self.ReceiveBeginPlay`)

(event `self.ReceiveTick`
  (params (DeltaSeconds :type "Float (single-precision)"))
  (`self.AddMovementInput` (`self.GetActorForwardVector`) 0.5 true))

(event `self.ReceiveHit`
  (params (MyComp :type "PrimitiveComponent Object Reference") (Other :type "Actor Object Reference") (OtherComp :type "PrimitiveComponent Object Reference") (bSelfMoved :type Boolean) (HitLocation :type "Object.Vector Structure") (HitNormal :type "Object.Vector Structure") (NormalImpulse :type "Object.Vector Structure") (Hit :type "EngineTypes.HitResult Structure (by ref)"))
  (bind _returnvalue (`GameplayStatics.GetObjectClass` (`self.HitActor`)))
  (set `self.HitActor` Other)
  (if (or (`KismetMathLibrary.ClassIsChildOf` _returnvalue "/Game/Blueprints/EggPlayer.EggPlayer_C") (`KismetMathLibrary.ClassIsChildOf` _returnvalue "/Script/EggletonProject.PaperEnemy"))
    (`GameplayStatics.ApplyDamage` (`self.HitActor`) 1.0))
  (`GameplayStatics.PlaySoundAtLocation` "/Game/Audio/Sound_Effects/Jump_Landed.Jump_Landed" (`self.K2_GetActorLocation`))
  (`self.K2_DestroyActor`))

(fn `UserConstructionScript`)